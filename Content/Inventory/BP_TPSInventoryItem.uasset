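; BP_TPSInventoryItem is an inventory pickup actor that displays its type as a shape and its score as text.
; Its construction script calls Init, which picks the mesh and sets the text from InventoryData.
; Init also applies a random palette color to a dynamic material and the text.
; EndPlay spawns the NS_Pickup Niagara effect at the actor's location, without checking why play ended.
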(event EventBeginPlay)

(event Collision|EventActorBeginOverlap
  (params (OtherActor :type Actor%20Object%20Reference)))

(event EventTick
  (params (DeltaSeconds :type Float%20%28single-precision%29)))

(event EventEndPlay
  (params (EndPlayReason :type EEndPlayReason%20Enum :default "Destroyed"))
  (Niagara|SpawnSystematLocation "/Game/Inventory/NS_Pickup.NS_Pickup" (Transformation|GetActorLocation)))

(fn ConstructionScript
  (CallFunction|Init))

(fn GenerateColor
  (return (.OutItem (Utilities|Array|Random (Variables|Default|GetColorPalette)))))

(fn Init
  (bind _inventorydata (Variables|Default|GetInventoryData))
  (Components|StaticMesh|SetStaticMesh (Variables|Default|GetStaticMesh) (Utilities|Select :Index (.type _inventorydata) :SPHERE "/Engine/BasicShapes/Sphere.Sphere" :CUBE "/Engine/BasicShapes/Cube.Cube" :CYLINDER "/Engine/BasicShapes/Cylinder.Cylinder" :CONE "/Engine/BasicShapes/Cone.Cone"))
  (Rendering|Components|TextRender|SetText (Variables|Default|GetTextRender) (Utilities|Text|ToText(Integer) (.score _inventorydata)))
  (bind _returnvalue (Rendering|Material|CreateDynamicMaterialInstance (Variables|Default|GetStaticMesh) 0 0 "None" :!class /Script/Engine.PrimitiveComponent))
  (bind _output_get (LocalVariables|SetItemColor (CallFunction|GenerateColor)))
  (Rendering|Material|SetVectorParameterValue _returnvalue "Color" _output_get :!class /Script/Engine.MaterialInstanceDynamic)
  (Rendering|Components|TextRender|SetTextRenderColor (Variables|Default|GetTextRender) (Math|Conversions|ToColor(LinearColor) (LocalVariables|GetItemColor))))